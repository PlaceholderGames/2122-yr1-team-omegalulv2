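; Projectile actor that damages enemies on contact and removes itself.
; When its Rew component begins an overlap, it casts the other actor to Flesh_Crab, Worm, Venomous and Spider, applying fixed damage through that class's DamageEnemy and destroying itself on a match.
; A delay started at BeginPlay destroys the projectile after a short lifetime.
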(event OnComponentBeginOverlap(rew)
  (params (OverlappedComponent :type Primitive%20Component%20Object%20Reference) (OtherActor :type Actor%20Object%20Reference) (OtherComp :type Primitive%20Component%20Object%20Reference) (OtherBodyIndex :type Integer) (bFromSweep :type Boolean) (SweepResult :type Hit%20Result%20Structure%20%28by%20ref%29))
  ;[1 1 1] Damage Mechanic
  (Utilities|FlowControl|Sequence
    (:then_0
      (bind _asflesh_crab (Utilities|Casting|CastToFlesh_Crab OtherActor))
      (Default|DamageEnemy _asflesh_crab 50)
      (Actor|DestroyActor))
    (:then_1
      (bind _asworm (Utilities|Casting|CastToWorm OtherActor))
      (Default|DamageEnemy _asworm 50)
      (Actor|DestroyActor))
    (:then_2
      (bind _asvenomous (Utilities|Casting|CastToVenomous OtherActor))
      (Default|DamageEnemy _asvenomous 50)
      (Actor|DestroyActor))
    (:then_3
      (bind _asspider (Utilities|Casting|CastToSpider OtherActor))
      (Default|DamageEnemy _asspider 50)
      (Actor|DestroyActor))))

(event EventBeginPlay
  ;[1 1 1] Removing Projectiles
  (Utilities|FlowControl|Delay 2.5)
  (Actor|DestroyActor))

(fn ConstructionScript)