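; Flipbook sprite enemy pawn that chases the main character and is destroyed when damage depletes its health.
; PawnSensing sightings set CanSeeEnemy and start AIMoveTo toward the player, with a retriggerable delay clearing the flag after sightings stop.
; Tick zeroes rotation and runs the State-based animation update, then overrides the flipbook with front or back according to Y velocity, showing front at zero.
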(event OnSeePawn(PawnSensing)
  (params (Pawn :type Pawn%20Object%20Reference))
  ;[1 1 1] Makes the AI walk to wards the player
  (bind _asmain_character (Utilities|Casting|CastToMainCharacter Pawn))
  (Utilities|FlowControl|Sequence
    (:then_0
      (Variables|Default|SetCan%20See%20Enemy? true)
      (AI|AIMoveTo self "0, 0, 0" _asmain_character 5.0 false))
    (:then_1
      (Utilities|FlowControl|RetriggerableDelay 0.6)
      (Variables|Default|SetCan%20See%20Enemy? false))))

(event Custom|Damage%20Enemy
  (params (Damage%20Taken :type Integer))
  ;[1 1 1] Damage
  (bind _output_get (Variables|Default|SetBad%20Guy%20Health (- (Variables|Default|GetBad%20Guy%20Health) Damage%20Taken)))
  (if (<= _output_get 0)
    (Actor|DestroyActor)))

(event Custom|Update%20Animation
  ;[1 1 1] Handle Animation
  (switch Utilities|FlowControl|Switch|SwitchonEnemy_State (Variables|Default|GetState)
    (:NewEnumerator0
      (Sprite|SetFlipbook (Variables|Default|GetSprite) "/Game/Blueprints/Enemy/enemy_front_flip.enemy_front_flip"))
    (:NewEnumerator1
      (Sprite|SetFlipbook (Variables|Default|GetSprite) "/Game/Blueprints/Enemy/enemy_back_flip.enemy_back_flip"))))

(event EventBeginPlay
  ;[1 1 1] Makes the AI walk to wards the player
)

(event EventTick
  (params (DeltaSeconds :type Float%20%28single-precision%29))
  ;[1 1 1] Update Animation
  (Utilities|FlowControl|Sequence
    (:then_0
      (Transformation|SetActorRotation self))
    (:then_1
      (CallFunction|UpdateAnimation)
      (Math|Float|CompareFloat (.Y (Math|Vector|BreakVector (Transformation|GetComponentVelocity (Variables|/Script/Engine.MovementComponent|GetUpdatedPrimitive (Pawn|GetMovementComponent))))) 0.0
        (:>
          (Sprite|SetFlipbook (Variables|Default|GetSprite) "/Game/Blueprints/Enemy/enemy_front_flip.enemy_front_flip" :!label _label))
        (:==
          (if true
            (goto _label)
            (else
              (Sprite|SetFlipbook (Variables|Default|GetSprite) "/Game/Blueprints/Enemy/enemy_back_flip.enemy_back_flip" :!label _label_2))))
        (:<
          (goto _label_2))))))

(fn ConstructionScript)