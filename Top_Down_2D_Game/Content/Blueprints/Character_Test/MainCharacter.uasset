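; MainCharacter is the player's Paper2D character, handling movement, shooting, score, damage and a pause menu.
; Axis input moves it, swaps directional flipbooks and sets FacingIndex, which picks the arrow component that projectiles spawn from.
; Damage_System, also wired to a Backslash key, lowers health and the health bar, opening the game-over level at zero.
; Tick's position comparison does nothing, and the state-based SetFlipBook function is not called here.
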(event Custom|Damage_System
  (params (Damage%20In :type Float%20%28single-precision%29))
  ;[1 1 1] Damage System
  (Variables|Default|SetIs%20Hit true)
  (Utilities|FlowControl|Sequence
    (:then_0
      (bind _output_get (Variables|Default|SetHealth%20Current (- (Variables|Default|GetHealth%20Current) Damage%20In)))
      (if (<= _output_get 0.0)
        (Actor|DestroyActor)
        (Game|OpenLevel(byName) "GameOver_Menu")))
    (:then_1
      (Variables|Default|SetHealth_Bar (- (Variables|Default|GetHealth_Bar) (Math|Float|Truncate (* (Variables|Default|GetMax%20Health) Damage%20In)))))))

(event Custom|Score_System
  (params (Score%20In :type Integer))
  ;[1 1 1] Score System
  (Variables|Default|SetScore (+ (Variables|Default|GetScore) Score%20In)))

(event EventTick
  (params (DeltaSeconds :type Float%20%28single-precision%29))
  ;[1 1 1] Tick - Update Animation
  (if (<= (- (.x (Transformation|GetWorldLocation (Variables|Default|GetSprite))) (.x (Transformation|GetActorLocation (Game|GetPlayerCharacter 0)))) 0.0)
    _))

(event Input|ActionEvents|InputActionPauseGame
  (params (Key :type Key%20Structure :default "None"))
  (bind _returnvalue (Game|GetPlayerController 0))
  ;[1 1 1] Pause / Unpause
  (:Pressed
    (Utilities|IsValid (Variables|Default|GetPause%20Menu%20REF)
      (:Is%20Valid
        _)
      (:Is%20Not%20Valid
        (bind _returnvalue_2 (UserInterface|CreateWidget "/Game/Menus/Pause_Menu_Widget.Pause_Menu_Widget_C"))
        (Variables|Default|SetPause%20Menu%20REF _returnvalue_2)))
    (if (Game|IsGamePaused)
      (Widget|RemovefromParent (Variables|Default|GetPause%20Menu%20REF))
      (Game|SetGamePaused false)
      (Variables|/Script/Engine.PlayerController|SetbShowMouseCursor _returnvalue false)
      (Input|SetInputModeGameOnly _returnvalue)
      (else
        (UserInterface|Viewport|AddtoViewport (Variables|Default|GetPause%20Menu%20REF) 0)
        (Game|SetGamePaused true)
        (Variables|/Script/Engine.PlayerController|SetbShowMouseCursor _returnvalue true)
        (Input|SetInputModeGameandUI _returnvalue (Variables|Default|GetPause%20Menu%20REF) "LockInFullscreen" false)))))

(event Input|ActionEvents|InputActionFire
  (params (Key :type Key%20Structure :default "None"))
  ;[1 1 1] Shooting
  (:Pressed
    (Game|SpawnActorfromClass "/Game/Blueprints/Projectile/Blueprint_Projectile.Blueprint_Projectile_C" (Transformation|GetWorldTransform (Utilities|Array|Get(acopy) (Utilities|Array|MakeArray (Variables|Default|GetArrow%20Right) (Variables|Default|GetArrow%20Left) (Variables|Default|GetArrow%20Up) (Variables|Default|GetArrow%20Down)) (Variables|Default|GetFacing%20%28Index%29))) "Undefined" 0 0)))

(event Input|AxisEvents|InputAxisMoveRight/Left
  (params (AxisValue :type Float%20%28single-precision%29))
  (bind _sprite (Variables|Default|GetSprite))
  ;[1 1 1] User input Right Left
  (Math|Float|CompareFloat AxisValue 0.0
    (:>
      (Variables|Default|SetIs%20Moving%20Right true)
      (Sprite|SetFlipbook _sprite "/Game/Blueprints/Character_Test/main_char_right.main_char_right")
      (Variables|Default|SetFacing%20%28Index%29 0))
    (:<
      (Variables|Default|SetIs%20Moving%20Right false)
      (Sprite|SetFlipbook _sprite "/Game/Blueprints/Character_Test/main_char_left.main_char_left")
      (Variables|Default|SetFacing%20%28Index%29 1)))
  (Pawn|Input|AddMovementInput "1.000000, 0, 0" AxisValue false))

(event Input|AxisEvents|InputAxisMoveUp/Down
  (params (AxisValue :type Float%20%28single-precision%29))
  (bind _sprite (Variables|Default|GetSprite))
  ;[1 1 1] User Input Up Down
  (Math|Float|CompareFloat AxisValue 0.0
    (:>
      (Variables|Default|SetIs%20Moving%20Up true)
      (Sprite|SetFlipbook _sprite "/Game/Blueprints/Character_Test/main_char_back.main_char_back")
      (Variables|Default|SetFacing%20%28Index%29 2))
    (:<
      (Variables|Default|SetIs%20Moving%20Up false)
      (Sprite|SetFlipbook _sprite "/Game/Blueprints/Character_Test/main_char_front.main_char_front")
      (Variables|Default|SetFacing%20%28Index%29 3)))
  (Pawn|Input|AddMovementInput "0,-1.000000, 0" AxisValue false))

(event Input|KeyboardEvents|Backslash
  (params (Key :type Key%20Structure :default "None"))
  ;[1 1 1] Damage System
  (:Pressed
    (Variables|Default|SetIs%20Hit true)
    (Utilities|FlowControl|Sequence
      (:then_0
        (bind _output_get (Variables|Default|SetHealth%20Current (- (Variables|Default|GetHealth%20Current) (stale Custom|Damage_System Damage%20In))))
        (if (<= _output_get 0.0)
          (Actor|DestroyActor)
          (Game|OpenLevel(byName) "GameOver_Menu")))
      (:then_1
        (Variables|Default|SetHealth_Bar (- (Variables|Default|GetHealth_Bar) (Math|Float|Truncate (* (Variables|Default|GetMax%20Health) (stale Custom|Damage_System Damage%20In)))))))))

(fn ConstructionScript)

(fn SetFlipBook
  (params (Next%20State :type AnimStates%20Enum :default "NewEnumerator1"))
  (Variables|Default|SetCurrent%20State Next%20State)
  (Sprite|SetFlipbook (Variables|Default|GetSprite) (Utilities|Select :Index (Variables|Default|GetCurrent%20State) :NewEnumerator1 (Variables|Default|GetFB%20%20Up%20-%20Back) :NewEnumerator2 (Variables|Default|GetFB%20Down%20-%20Front) :NewEnumerator3 0 :NewEnumerator4 0))
  (return))