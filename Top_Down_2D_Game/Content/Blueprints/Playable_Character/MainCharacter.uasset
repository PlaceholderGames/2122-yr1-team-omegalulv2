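; Playable 2D flipbook character that moves, fires projectiles and toggles the pause menu.
; Two input axes drive movement along world X and Y, directly swapping directional flipbooks and setting movement flags.
; Fire spawns a projectile at Arrow1; its retriggerable delays lead nowhere.
; Pause lazily creates the widget and switches input mode; the Tick animation check is empty, and the state-based SetFlipBook function is never called here.
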(event EventTick
  (params (DeltaSeconds :type Float%20%28single-precision%29))
  ;[1 1 1] Tick - Update Animation
  (if (<= (- (.x (Transformation|GetWorldLocation (Variables|Default|GetSprite))) (.x (Transformation|GetActorLocation (Game|GetPlayerCharacter 0)))) 0.0)
    _))

(event Input|ActionEvents|InputActionPauseGame
  (params (Key :type Key%20Structure))
  (bind _returnvalue (Game|GetPlayerController 0))
  ;[1 1 1] Pause / Unpause
  (:Pressed
    (Utilities|IsValid (Variables|Default|GetPause%20Menu%20REF)
      (:Is%20Valid
        _)
      (:Is%20Not%20Valid
        (bind _returnvalue_2 (UserInterface|CreateWidget "/Game/Menus/Pause_Menu_Widget.Pause_Menu_Widget_C"))
        (Variables|Default|SetPause%20Menu%20REF _returnvalue_2)))
    (if (Game|IsGamePaused)
      (Widget|RemovefromParent (Variables|Default|GetPause%20Menu%20REF))
      (Game|SetGamePaused false)
      (Variables|/Script/Engine.PlayerController|SetbShowMouseCursor _returnvalue false)
      (Input|SetInputModeGameOnly _returnvalue)
      (else
        (UserInterface|Viewport|AddtoViewport (Variables|Default|GetPause%20Menu%20REF) 0)
        (Game|SetGamePaused true)
        (Variables|/Script/Engine.PlayerController|SetbShowMouseCursor _returnvalue true)
        (Input|SetInputModeGameandUI _returnvalue (Variables|Default|GetPause%20Menu%20REF) "LockInFullscreen" false)))))

(event Input|ActionEvents|InputActionFire
  (params (Key :type Key%20Structure))
  ;[1 1 1] Shooting
  (:Pressed
    (Game|SpawnActorfromClass "/Game/Blueprints/Projectile/Blueprint_Projectile.Blueprint_Projectile_C" (Transformation|GetWorldTransform (Variables|Default|GetArrow1)) "Undefined" 0 0)
    (Utilities|FlowControl|RetriggerableDelay 2.0))
  (:Released
    (Utilities|FlowControl|RetriggerableDelay 2.0)))

(event Input|AxisEvents|InputAxisMoveRight/Left
  (params (AxisValue :type Float%20%28single-precision%29))
  (bind _sprite (Variables|Default|GetSprite))
  ;[1 1 1] User input Right Left
  (Math|Float|CompareFloat AxisValue 0.0
    (:>
      (Variables|Default|SetIs%20Moving%20Right true)
      (Sprite|SetFlipbook _sprite "/Game/Blueprints/Playable_Character/main_char_right.main_char_right"))
    (:<
      (Variables|Default|SetIs%20Moving%20Right false)
      (Sprite|SetFlipbook _sprite "/Game/Blueprints/Playable_Character/main_char_left.main_char_left")))
  (Pawn|Input|AddMovementInput "1.000000, 0, 0" AxisValue false))

(event Input|AxisEvents|InputAxisMoveUp/Down
  (params (AxisValue :type Float%20%28single-precision%29))
  (bind _sprite (Variables|Default|GetSprite))
  ;[1 1 1] User Input Up Down
  (Math|Float|CompareFloat AxisValue 0.0
    (:>
      (Variables|Default|SetIs%20Moving%20Up true)
      (Sprite|SetFlipbook _sprite "/Game/Blueprints/Playable_Character/main_char_back.main_char_back"))
    (:<
      (Variables|Default|SetIs%20Moving%20Up false)
      (Sprite|SetFlipbook _sprite "/Game/Blueprints/Playable_Character/main_char_front.main_char_front")))
  (Pawn|Input|AddMovementInput "0,-1.000000, 0" AxisValue false))

(fn ConstructionScript)

(fn SetFlipBook
  (params (Next%20State :type AnimStates%20Enum :default "NewEnumerator1"))
  (Variables|Default|SetCurrent%20State Next%20State)
  (Sprite|SetFlipbook (Variables|Default|GetSprite) (Utilities|Select :Index (Variables|Default|GetCurrent%20State) :NewEnumerator1 (Variables|Default|GetFB%20%20Up%20-%20Back) :NewEnumerator2 (Variables|Default|GetFB%20Down%20-%20Front) :NewEnumerator3 0 :NewEnumerator4 0))
  (return))